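; BP_Catapult is a physics-driven catapult that launches cannonballs and must be reloaded between shots.
; Shoot, when loaded, pitches the PhysicsConstraint's angular orientation target to swing the arm and clears the Load flag, otherwise printing an empty warning.
; Reload resets that target, calls MoveComponentTo on SpoonMesh, and starts a short timer that spawns a BP_Cannonball at the Spawn transform and sets Load.
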(event `Shoot`
  (if (`self.bLoad`)
    (`PhysicsConstraintComponent.SetAngularOrientationTarget` (`self.PhysicsConstraint`) (`KismetMathLibrary.MakeRotator` 0.0 90.0))
    (`KismetSystemLibrary.PrintString` "Catapult shot!")
    (set `self.bLoad` false)
    (else
      (`KismetSystemLibrary.PrintString` "Catapult empty! Need to reload!"))))

(event `Reload`
  (bind _spoonmesh (`self.SpoonMesh`))
  (`PhysicsConstraintComponent.SetAngularOrientationTarget` (`self.PhysicsConstraint`) (`KismetMathLibrary.MakeRotator` 0.0 0.0))
  (`KismetSystemLibrary.MoveComponentTo` _spoonmesh (`SceneComponent.RelativeLocation` _spoonmesh))
  (bind _returnvalue (`KismetSystemLibrary.K2_SetTimerDelegate` (delegate `SpawnBall`) 2.0))
  (set `self.ReloadTimer` _returnvalue))

(event `SpawnBall`
  (`|SpawnActorFromClass` "/Game/HW_03/Blueprints/Cannonball/BP_Cannonball.BP_Cannonball_C" (`SceneComponent.K2_GetComponentToWorld` (`self.Spawn`)) "AlwaysSpawn" "MultiplyWithRoot" null null)
  (set `self.bLoad` true)
  (`KismetSystemLibrary.K2_ClearAndInvalidateTimerHandle` (`self.ReloadTimer`)))

(fn `UserConstructionScript`)